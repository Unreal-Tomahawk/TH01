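; Map helper Blueprint for block building: it snaps new actors flush onto the faces of existing ones and stores a per-actor outline flag.
; Half-extents come from static mesh bounds, using a temporary spawn for classes, to identify hit faces and compute rotation-aware neighbor transforms and boxes.
; The Testing routine spawns bricks at line-trace hits, falling back to a capsule trace that tests hidden-face boxes against the camera's sight line.
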(fn `Actor Is Type`
  (params (Actor :type "Actor Object Reference") (Type1 :type String) (Type2 :type String))
  (returns (`Is Valid` :type Boolean))
  (bind _asbase_obj_a1_blueprint (cast `/Game/Blueprints/Actors/BaseObjA1_Blueprint` Actor)
    (:`then`
      (if (`KismetStringLibrary.EqualEqual_StrStr` Type1 "*")
        (return true)
        (elif (`KismetStringLibrary.EqualEqual_StrStr` Type1 (`/Game/Blueprints/Actors/BaseObjA1_Blueprint.type1` _asbase_obj_a1_blueprint))
          (if (`KismetStringLibrary.EqualEqual_StrStr` Type2 "*")
            (return true)
            (elif (`KismetStringLibrary.EqualEqual_StrStr` Type2 (`/Game/Blueprints/Actors/BaseObjA1_Blueprint.type2` _asbase_obj_a1_blueprint))
              (return true)
              (else
                (return false))))
          (else
            (return false)))))
    (:`CastFailed`
      (return false))))

(fn `Create Actor Snap`
  (params (`New Object Class` :type "Actor Class Reference") (`Target Actor` :type "Actor Object Reference") (`Hit Point` :type "Vector Structure"))
  (returns (`New Actor` :type "Actor Object Reference"))
  (bind _snap_transform (`self.Get Actor Snap Transform` `New Object Class` `Target Actor` `Hit Point`))
  (bind _returnvalue (`|SpawnActorFromClass` `New Object Class` _snap_transform "Undefined" "OverrideRootScale" null null))
  (return _returnvalue))

(fn `Get Actor 6Box by Class`
  (params (targetActor :type "Actor Object Reference") (`6BoxClass` :type "Actor Class Reference"))
  (returns (`6Box` :type "Array of TamWorldBox Structure"))
  (bind _extent (`self.Get Actor Size By Class` `6BoxClass`))
  (bind _x (.x _extent))
  (bind _y (.y _extent))
  (bind _z (.z _extent))
  (bind _surface_dist_transform (`self.Get Actor Surface Dist Transform` targetActor "Top" _z))
  (bind _surface_dist_transform_2 (`self.Get Actor Surface Dist Transform` targetActor "Bottom" _z))
  (bind _surface_dist_transform_3 (`self.Get Actor Surface Dist Transform` targetActor "Left" _y))
  (bind _surface_dist_transform_4 (`self.Get Actor Surface Dist Transform` targetActor "Right" _y))
  (bind _surface_dist_transform_5 (`self.Get Actor Surface Dist Transform` targetActor "Front" _x))
  (bind _surface_dist_transform_6 (`self.Get Actor Surface Dist Transform` targetActor "Back" _x))
  (return (`|MakeArray` (make `TamWorldBox` (.location _surface_dist_transform) (.rotation _surface_dist_transform) _extent) (make `TamWorldBox` (.location _surface_dist_transform_2) (.rotation _surface_dist_transform_2) _extent) (make `TamWorldBox` (.location _surface_dist_transform_3) (.rotation _surface_dist_transform_3) _extent) (make `TamWorldBox` (.location _surface_dist_transform_4) (.rotation _surface_dist_transform_4) _extent) (make `TamWorldBox` (.location _surface_dist_transform_5) (.rotation _surface_dist_transform_5) _extent) (make `TamWorldBox` (.location _surface_dist_transform_6) (.rotation _surface_dist_transform_6) _extent))))

(fn `Get Actor Far 3Box by Class`
  (params (targetActor :type "Actor Object Reference") (`6BoxClass` :type "Actor Class Reference") (cameraPosition :type "Vector Structure"))
  (returns (`3Box` :type "Array of TamWorldBox Structure"))
  (bind _extent (`self.Get Actor Size By Class` `6BoxClass`))
  (bind _x (.x _extent))
  (bind _y (.y _extent))
  (bind _z (.z _extent))
  (bind _surface_dist_transform (`self.Get Actor Surface Dist Transform` targetActor "Top" _z))
  (bind _surface_dist_transform_2 (`self.Get Actor Surface Dist Transform` targetActor "Bottom" _z))
  (bind _surface_dist_transform_3 (`self.Get Actor Surface Dist Transform` targetActor "Left" _y))
  (bind _surface_dist_transform_4 (`self.Get Actor Surface Dist Transform` targetActor "Right" _y))
  (bind _surface_dist_transform_5 (`self.Get Actor Surface Dist Transform` targetActor "Front" _x))
  (bind _surface_dist_transform_6 (`self.Get Actor Surface Dist Transform` targetActor "Back" _x))
  (bind _location (.location _surface_dist_transform))
  (bind _location_2 (.location _surface_dist_transform_2))
  (bind _location_3 (.location _surface_dist_transform_3))
  (bind _location_4 (.location _surface_dist_transform_4))
  (bind _location_5 (.location _surface_dist_transform_5))
  (bind _location_6 (.location _surface_dist_transform_6))
  (return (`|MakeArray` (select `bool` (< (`KismetMathLibrary.Vector_Distance` cameraPosition _location) (`KismetMathLibrary.Vector_Distance` cameraPosition _location_2)) :`false` (make `TamWorldBox` _location (.rotation _surface_dist_transform) _extent) :`true` (make `TamWorldBox` _location_2 (.rotation _surface_dist_transform_2) _extent)) (select `bool` (< (`KismetMathLibrary.Vector_Distance` cameraPosition _location_3) (`KismetMathLibrary.Vector_Distance` cameraPosition _location_4)) :`false` (make `TamWorldBox` _location_3 (.rotation _surface_dist_transform_3) _extent) :`true` (make `TamWorldBox` _location_4 (.rotation _surface_dist_transform_4) _extent)) (select `bool` (< (`KismetMathLibrary.Vector_Distance` cameraPosition _location_5) (`KismetMathLibrary.Vector_Distance` cameraPosition _location_6)) :`false` (make `TamWorldBox` _location_5 (.rotation _surface_dist_transform_5) _extent) :`true` (make `TamWorldBox` _location_6 (.rotation _surface_dist_transform_6) _extent)))))

(fn `Get Actor Size`
  (params (Actor :type "Actor Object Reference"))
  (returns (Extent :type "Vector Structure"))
  (bind _asstatic_mesh_component (cast `StaticMeshComponent` (`Actor.RootComponent` Actor)))
  (bind (_min _max) (break `Box` (`StaticMesh.GetBoundingBox` (`StaticMeshComponent.StaticMesh` _asstatic_mesh_component))))
  (return (* (* (- _max _min) (.scale (`self.GetTransform` Actor))) 0.5)))

(fn `Get Actor Size By Class`
  (params (`Actor Class` :type "Actor Class Reference"))
  (returns (Extent :type "Vector Structure"))
  (bind _returnvalue (`|SpawnActorFromClass` `Actor Class` (`KismetMathLibrary.MakeTransform` (0.0 0.0 0.0)) "Undefined" "OverrideRootScale" null null))
  (bind _extent (`self.Get Actor Size` _returnvalue))
  (`self.K2_DestroyActor` _returnvalue)
  (return _extent))

(fn `Get Actor Snap Transform`
  (params (`New Object Class` :type "Actor Class Reference") (`Target Actor` :type "Actor Object Reference") (`Hit Point` :type "Vector Structure"))
  (returns (`Snap Transform` :type "Transform Structure"))
  (bind _surface_name (`self.Get Point at Actor Which Surface` `Target Actor` `Hit Point`))
  (bind _extent (`self.Get Actor Size By Class` `New Object Class`))
  (switch `string` _surface_name
    (:`top`
      _)
    (:`bottom`
      _)
    (:`left`
      (bind _surface_dist_transform (`self.Get Actor Surface Dist Transform` `Target Actor` _surface_name (.y _extent) :!label _label))
      (return _surface_dist_transform))
    (:`right`
      (goto _label))
    (:`front`
      (bind _surface_dist_transform_2 (`self.Get Actor Surface Dist Transform` `Target Actor` _surface_name (.x _extent) :!label _label_2))
      (return _surface_dist_transform_2))
    (:`back`
      (goto _label_2)))
  (bind _surface_dist_transform_3 (`self.Get Actor Surface Dist Transform` `Target Actor` _surface_name (.z _extent)))
  (return _surface_dist_transform_3))

(fn `Get Actor Surface Dist Transform`
  (params (Actor :type "Actor Object Reference") (`Surface Name` :type String) (Distance :type "Float (double-precision)"))
  (returns (`Surface Dist Transform` :type "Transform Structure"))
  (bind _face_center_add_distance_vector (`self.Get Actor Surface Vector` Actor `Surface Name` Distance))
  (return (`KismetMathLibrary.MakeTransform` (+ _face_center_add_distance_vector (.location (`self.GetTransform` Actor))) (.rotation (`self.GetTransform` Actor)))))

(fn `Get Actor Surface Vector`
  (params (Actor :type "Actor Object Reference") (`Surface Name` :type String) (Distance :type "Float (double-precision)"))
  (returns (`Face Center Add Distance Vector` :type "Vector Structure"))
  (bind _returnvalue (`self.GetActorUpVector` Actor))
  (bind _returnvalue_2 (`self.GetActorRightVector` Actor))
  (bind _returnvalue_3 (`self.GetActorForwardVector` Actor))
  (bind _extent (`self.Get Actor Size` Actor))
  (switch `string` `Surface Name`
    (:`top`
      (bind _returnvalue_4 (+ (.z _extent) Distance))
      (return (* _returnvalue _returnvalue_4)))
    (:`bottom`
      (return (* (* _returnvalue -1.0) _returnvalue_4)))
    (:`left`
      (bind _returnvalue_5 (+ (.y _extent) Distance))
      (return (* (* _returnvalue_2 -1.0) _returnvalue_5)))
    (:`right`
      (return (* _returnvalue_2 _returnvalue_5)))
    (:`front`
      (bind _returnvalue_6 (+ (.x _extent) Distance))
      (return (* _returnvalue_3 _returnvalue_6)))
    (:`back`
      (return (* (* _returnvalue_3 -1.0) _returnvalue_6)))))

(fn `Get Outline Enabled`
  (params (actor :type "Actor Object Reference"))
  (returns (outlineEnabled :type Boolean))
  (bind _objectcustomdata (`self.objectCustomData`))
  (for _array_element _objectcustomdata
    (bind (_actor _outlineenabled) (break `/Game/Blueprints/objectCustomDataItem` _array_element))
    (if (== _actor actor)
      (return _outlineenabled)))
  (`KismetArrayLibrary.Array_Add` _objectcustomdata (make `/Game/Blueprints/objectCustomDataItem` actor))
  (return false))

(fn `Get Point at Actor Which Surface`
  (params (Actor :type "Actor Object Reference") (Point :type "Vector Structure"))
  (returns (`Surface Name` :type String))
  (bind _x (.x (`KismetMathLibrary.GreaterGreater_VectorRotator` (- Point (.location (`self.GetTransform` Actor))) (`KismetMathLibrary.NegateRotator` (.rotation (`self.GetTransform` Actor))))))
  (bind _y (.y (`KismetMathLibrary.GreaterGreater_VectorRotator` (- Point (.location (`self.GetTransform` Actor))) (`KismetMathLibrary.NegateRotator` (.rotation (`self.GetTransform` Actor))))))
  (bind _z (.z (`KismetMathLibrary.GreaterGreater_VectorRotator` (- Point (.location (`self.GetTransform` Actor))) (`KismetMathLibrary.NegateRotator` (.rotation (`self.GetTransform` Actor))))))
  (bind _extent (`self.Get Actor Size` Actor))
  (if (`KismetMathLibrary.NearlyEqual_FloatFloat` (.z _extent) _z 0.001)
    (return "Top")
    (elif (`KismetMathLibrary.NearlyEqual_FloatFloat` (.z (* _extent -1.0)) _z 0.001)
      (return "Bottom")
      (elif (`KismetMathLibrary.NearlyEqual_FloatFloat` (.y (* _extent -1.0)) _y 0.001)
        (return "Left")
        (elif (`KismetMathLibrary.NearlyEqual_FloatFloat` (.y _extent) _y 0.001)
          (return "Right")
          (elif (`KismetMathLibrary.NearlyEqual_FloatFloat` (.x _extent) _x 0.001)
            (return "Front")
            (elif (`KismetMathLibrary.NearlyEqual_FloatFloat` (.x (* _extent -1.0)) _x 0.001)
              (return "Back")
              (else
                (return "")))))))))

(fn `Get User Signt Line Point`
  (params (distance :type "Float (double-precision)"))
  (returns (point :type "Vector Structure"))
  (bind _camera (`self.camera`))
  (return (+ (`SceneComponent.K2_GetComponentLocation` _camera) (`KismetMathLibrary.GreaterGreater_VectorRotator` (`KismetMathLibrary.MakeVector` distance) (`SceneComponent.K2_GetComponentRotation` _camera)))))

(fn `getActorSnapBox`
  (params (`Target Actor` :type "Actor Object Reference") (`New Object Class` :type "Actor Class Reference") (`Surface Name` :type String))
  (returns (TamWorldBox :type "TamWorldBox Structure"))
  (bind _extent (`self.Get Actor Size By Class` `New Object Class`))
  (switch `string` `Surface Name`
    (:`Front`
      (bind _x (.x _extent))
      (bind _y (.y _extent))
      (bind _z (.z _extent))
      (bind _surface_dist_transform (`self.Get Actor Surface Dist Transform` `Target Actor` `Surface Name` _x))
      (return (make `TamWorldBox` (.location _surface_dist_transform) (.rotation _surface_dist_transform) _extent)))
    (:`Back`
      (bind _surface_dist_transform_2 (`self.Get Actor Surface Dist Transform` `Target Actor` `Surface Name` _x))
      (return (make `TamWorldBox` (.location _surface_dist_transform_2) (.rotation _surface_dist_transform_2) _extent)))
    (:`Right`
      (bind _surface_dist_transform_3 (`self.Get Actor Surface Dist Transform` `Target Actor` `Surface Name` _y))
      (return (make `TamWorldBox` (.location _surface_dist_transform_3) (.rotation _surface_dist_transform_3) _extent)))
    (:`Left`
      (bind _surface_dist_transform_4 (`self.Get Actor Surface Dist Transform` `Target Actor` `Surface Name` _y))
      (return (make `TamWorldBox` (.location _surface_dist_transform_4) (.rotation _surface_dist_transform_4) _extent)))
    (:`Top`
      (bind _surface_dist_transform_5 (`self.Get Actor Surface Dist Transform` `Target Actor` `Surface Name` _z))
      (return (make `TamWorldBox` (.location _surface_dist_transform_5) (.rotation _surface_dist_transform_5) _extent)))
    (:`Bottom`
      (bind _surface_dist_transform_6 (`self.Get Actor Surface Dist Transform` `Target Actor` `Surface Name` _z))
      (return (make `TamWorldBox` (.location _surface_dist_transform_6) (.rotation _surface_dist_transform_6) _extent)))))

(fn `Set Outline Enabled`
  (params (actor :type "Actor Object Reference") (`outline enabled` :type Boolean))
  (bind _objectcustomdata (`self.objectCustomData`))
  (for (_array_element _array_index) _objectcustomdata
    (if (== actor (`.actor_2_EB5530E34BD5E2E5D30D119C33645B14` (break `/Game/Blueprints/objectCustomDataItem` _array_element)))
      (bind _structout (setmembers `/Game/Blueprints/objectCustomDataItem` :`StructRef` _array_element :`outlineEnabled` `outline enabled`))
      (`KismetArrayLibrary.Array_Set` (`self.objectCustomData`) _array_index _structout)
      (return)))
  (`KismetArrayLibrary.Array_Add` _objectcustomdata (make `/Game/Blueprints/objectCustomDataItem` actor `outline enabled`))
  (return))

(fn `Testing`
  (locals (boxArray :type "Array of TamWorldBox Structure"))
  (bind _boxarray (`local.boxArray`))
  (bind _point (`self.Get User Signt Line Point` 150.0))
  (bind _point_2 (`self.Get User Signt Line Point` 20000.0))
  ;[0.4728 0.2257 1] 接触撞击优先
  (bind (_outhit _returnvalue) (`KismetSystemLibrary.LineTraceSingle` _point _point_2 "TraceTypeQuery1"))
  (if _returnvalue
    (bind (_bblockinghit _binitialoverlap _time _distance _location _impactpoint _normal _impactnormal _physmat _hitactor) (`GameplayStatics.BreakHitResult` _outhit))
    (bind _is_valid (`self.Actor Is Type` _hitactor "base" "brick"))
    (if _is_valid
      (`self.Create Actor Snap` "/Game/Blueprints/Actors/BaseObjA1_Blueprint.BaseObjA1_Blueprint_C" _hitactor _location)
      (else
        ;[0.2395 0.5426 1] 获取非接触撞击点
        (bind _extent (`self.Get Actor Size By Class` "/Game/Blueprints/Actors/BaseObjA1_Blueprint.BaseObjA1_Blueprint_C" :!label _label))
        (bind _outhits (`KismetSystemLibrary.CapsuleTraceMultiForObjects` _point (`KismetMathLibrary.SelectVector` _location _point_2 _returnvalue) (`KismetMathLibrary.FMin` (.x _extent) (.y _extent) (.z _extent)) 0.0 (`|MakeArray` "ObjectTypeQuery1" "ObjectTypeQuery2" "ObjectTypeQuery4" :!type "EObjectTypeQuery Enum")))
        (bind _returnvalue_2 (`KismetArrayLibrary.Array_Length` _outhits))
        (for _index (range 1 (+ _returnvalue_2 1)) :!label _label_2
          (bind (_bblockinghit_2 _binitialoverlap_2 _time_2 _distance_2 _location_2 _impactpoint_2 _normal_2 _impactnormal_2 _physmat_2 _hitactor_2) (`GameplayStatics.BreakHitResult` (`|GetArrayItem` _outhits (- _returnvalue_2 _index))))
          (bind _is_valid_2 (`self.Actor Is Type` _hitactor_2 "base" "brick"))
          (if _is_valid_2
            (bind _point_3 (`self.Get User Signt Line Point` 0.0))
            (bind _tamworldbox (`/Game/Blueprints/TamClass/Etc/Actor.getActorBox` _hitactor_2))
            (bind _array (`/Game/Blueprints/TamClass/Math/TamWorldBox.getInvisibleSurfaceName` _tamworldbox _point_3))
            (for _array_element _array
              (`KismetSystemLibrary.PrintString` "Hello")
              (bind _tamworldbox_2 (`self.getActorSnapBox` _hitactor_2 "/Game/Blueprints/Actors/BaseObjA1_Blueprint.BaseObjA1_Blueprint_C" _array_element))
              (`KismetArrayLibrary.Array_Add` _boxarray _tamworldbox_2)
              (for _array_element_2 _boxarray
                (bind (_position _rotation _extent_2) (break `TamWorldBox` _array_element_2))
                (`KismetSystemLibrary.DrawDebugBox` _position _extent_2 (struct :`R` 0.904661 :`G` 0.564712 :`B` 0.205079 :`A` 1.0) _rotation 5.0 2.0)
                (bind _point_4 (`self.Get User Signt Line Point` 150.0))
                (bind _point_5 (`self.Get User Signt Line Point` 20000.0))
                (bind (_segmentintersection _extlineintersection) (`/Game/Blueprints/TamClass/Math/TamWorldBox.Intersection Line` _array_element_2 (make `TamLine` _point_4 _point_5)))
                (if (or _segmentintersection _extlineintersection)
                  (bind (_position_2 _rotation_2) (break `TamWorldBox` _array_element_2))
                  (`|SpawnActorFromClass` "/Game/Blueprints/Actors/BaseObjA1_Blueprint.BaseObjA1_Blueprint_C" (`KismetMathLibrary.MakeTransform` _position_2 _rotation_2) "Undefined" "OverrideRootScale" null null)
                  (break)))
              (`KismetSystemLibrary.DrawDebugPoint` _impactpoint_2 20.0 (struct :`G` 0.854167 :`B` 0.267127 :`A` 1.0) 10.0)
              (goto _label_2 :!via `Break`))))))
    (else
      (goto _label))))

(fn `UserConstructionScript`)